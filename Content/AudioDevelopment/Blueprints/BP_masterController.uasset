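; Master controller for a music-note puzzle that checks an Input array of notes against an Answer array, all on BeginPlay.
; It writes into Input and appends a MusicBox reference, with a loop over Input wired back into that same append.
; Nested loops then compare every Answer element with every Input element, printing "correct" on a match and clearing Input on any mismatch, so note order is not checked.
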(event `self.ReceiveBeginPlay`
  (bind _input (`self.Input`))
  ;[1 1 1] adds music notes to the input array
  (set `self.set array length` (`KismetArrayLibrary.Array_Length` (`self.Input`)))
  (`KismetArrayLibrary.Array_Set` _input (+ (`self.inputIndex`) 1) (`self.inputIndex`))
  (`KismetArrayLibrary.Array_Add` _input (`/Game/AudioDevelopment/Blueprints/BP_MusicalNote.Music box` (`self.Target`)) :!label _label)
  (bind _output_get (set `self.Input` (`self.Input`)))
  (for (_ _array_index) _output_get
    (goto _label))
  (`KismetSystemLibrary.PrintString` (`KismetStringLibrary.Conv_IntToString` _array_index))
  ;[1 1 1] compares the arrays to see if the answer is right
  (for _array_element (`self.Answer`)
    (for _array_element_2 (`self.Input`)
      (if (== _array_element_2 _array_element)
        (`KismetSystemLibrary.PrintString` "correct")
        (else
          (`KismetArrayLibrary.Array_Clear` (`self.Input`))
          (`KismetSystemLibrary.PrintString` "false"))))))

(fn `UserConstructionScript`)